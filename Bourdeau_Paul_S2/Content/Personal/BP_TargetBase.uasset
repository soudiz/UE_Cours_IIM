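; Base shooting-target actor that awards points by hit zone and target type, including a penalty type with negative scores.
; The construction script creates a dynamic material on the skeletal mesh, then UpdateTargetProperties sets head and body point values and BodyColor from TargetType.
; A hit on the head or body collision broadcasts the matching points through the TargetHasBeenHit dispatcher and destroys the actor.
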(event `self.HeadCollision.OnComponentHit`
  (params (HitComponent :type "PrimitiveComponent Object Reference") (OtherActor :type "Actor Object Reference") (OtherComp :type "PrimitiveComponent Object Reference") (NormalImpulse :type "Vector Structure") (Hit :type "HitResult Structure (by ref)"))
  (`self.TargetHasBeenHit` (`self.PointsValueHeadshot`))
  (`self.K2_DestroyActor`))

(event `self.BodyCollision.OnComponentHit`
  (params (HitComponent :type "PrimitiveComponent Object Reference") (OtherActor :type "Actor Object Reference") (OtherComp :type "PrimitiveComponent Object Reference") (NormalImpulse :type "Vector Structure") (Hit :type "HitResult Structure (by ref)"))
  (`self.TargetHasBeenHit` (`self.PointsValueBodyShot`))
  (`self.K2_DestroyActor`))

(fn `UpdateTargetProperties`
  (switch `int` (`self.TargetType`)
    (:`0`
      (set `self.PointsValueHeadshot` 200)
      (set `self.PointsValueBodyShot` 100)
      (`MaterialInstanceDynamic.SetVectorParameterValue` (`self.SK_Mesh_Material`) "BodyColor" (struct :`R` 0.945384 :`G` 0.35686 :`B` 1.0 :`A` 1.0)))
    (:`1`
      (set `self.PointsValueHeadshot` 500)
      (set `self.PointsValueBodyShot` 200)
      (`MaterialInstanceDynamic.SetVectorParameterValue` (`self.SK_Mesh_Material`) "BodyColor" (struct :`R` 0.166444 :`G` 0.645833 :`B` 0.14038 :`A` 1.0)))
    (:`2`
      (set `self.PointsValueHeadshot` 400)
      (set `self.PointsValueBodyShot` 100)
      (`MaterialInstanceDynamic.SetVectorParameterValue` (`self.SK_Mesh_Material`) "BodyColor" (struct :`R` 0.148003 :`G` 0.488812 :`B` 0.645833 :`A` 1.0)))
    (:`3`
      (set `self.PointsValueHeadshot` -100)
      (set `self.PointsValueBodyShot` -200)
      (`MaterialInstanceDynamic.SetVectorParameterValue` (`self.SK_Mesh_Material`) "BodyColor" (struct :`R` 0.645833 :`G` 0.087416 :`B` 0.093841 :`A` 1.0)))))

(fn `UserConstructionScript`
  (bind _skeletalmesh (`self.SkeletalMesh`))
  (bind _returnvalue (`PrimitiveComponent.CreateDynamicMaterialInstance` _skeletalmesh 0 (`PrimitiveComponent.GetMaterial` _skeletalmesh 0) "None"))
  (set `self.SK_Mesh_Material` _returnvalue)
  (`self.UpdateTargetProperties`))